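; BP_EnemyAI is the enemy AI controller logic that sets up blackboard BB_Enemy and runs behavior tree BT_Enemy.
; On BeginPlay it stores the player pawn and the distance settings from DT_Enemy's NpcBase row, starting the tree only if that row is found.
; Perception updates fill the EnemyActor key with a successfully sensed BP_Enemy, only while that key holds no valid actor.
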(event OnPerceptionUpdated(AIPerception)
  (params (UpdatedActors :type Array%20of%20Actor%20Object%20References))
  (Utilities|IsValid (AI|Components|Blackboard|GetValueasObject (Variables|Default|GetBlackboard) (Utilities|Name|MakeLiteralName "EnemyActor"))
    (:Is%20Not%20Valid
      (bind _array_element (Utilities|Array|ForEachLoopwithBreak UpdatedActors :!label _label)
        (:LoopBody
          (bind _info (Class|AIPerceptionComponent|GetActorsPerception (Variables|Default|GetAIPerception) _array_element))
          (if (.bSuccessfullySensed (Utilities|Struct|BreakAIStimulus (Utilities|Array|Get(acopy) (.LastSensedStimuli (Utilities|Struct|BreakActorPerceptionBlueprintInfo _info)))))
            (bind _asbp_enemy (Utilities|Casting|CastToBP_Enemy _array_element))
            (AI|Components|Blackboard|SetValueasObject (Variables|Default|GetBlackboard) (Utilities|Name|MakeLiteralName "EnemyActor") _asbp_enemy)
            (goto _label Break)))))))

(event EventBeginPlay
  (Class|AIController|UseBlackboard "/Game/Character/Nakajima/Enemy/BB_Enemy.BB_Enemy")
  (AI|Components|Blackboard|SetValueasObject (Variables|Default|GetBlackboard) (Utilities|Name|MakeLiteralName "PlayerActor") (Game|Player|GetPlayerPawn 0))
  (bind _returnvalue (Utilities|GetDataTableRow "/Game/Character/Nakajima/Enemy/DT_Enemy.DT_Enemy" "NpcBase")
    (:then
      (AI|Components|Blackboard|SetValueasFloat (Variables|Default|GetBlackboard) (Utilities|Name|MakeLiteralName "DistanceToPlayer") (.distancetoplayer _returnvalue))
      (AI|Components|Blackboard|SetValueasFloat (Variables|Default|GetBlackboard) (Utilities|Name|MakeLiteralName "DistanceToEnemy") (.distancetoenemy _returnvalue))
      (AI|RunBehaviorTree "/Game/Character/Nakajima/Enemy/BT_Enemy.BT_Enemy"))))

(event EventTick
  (params (DeltaSeconds :type Float%20%28single-precision%29)))

(fn ConstructionScript)